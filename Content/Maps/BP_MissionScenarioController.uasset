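; Mission scenario controller that handles the end-of-mission presentation when OnMissionFinished fires.
; It caches success, score, drones used and time, then after a short delay plays the WBP_MissionEndTransition fade.
; After a second delay it creates WBP_MissionResult with those cached values and itself as controller, then removes the transition.
; Finally it pauses the game, shows the mouse cursor and switches input to UI only.
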(event EventBeginPlay)

(event Collision|EventActorBeginOverlap
  (params (OtherActor :type Actor%20Object%20Reference)))

(event EventTick
  (params (DeltaSeconds :type Float%20%28single-precision%29)))

(event EventOnMissionFinished
  (params (bSuccess :type Boolean) (FinalScore :type Integer) (FinalUsedDrones :type Integer) (FinalTimeSeconds :type Float%20%28single-precision%29))
  (bind _returnvalue (Game|GetPlayerController 0))
  (Variables|Default|SetCachedMissionSuccess bSuccess)
  (Variables|Default|SetCachedFinalScore FinalScore)
  (Variables|Default|SetCachedFinalUsedDrones FinalUsedDrones)
  (Variables|Default|SetCachedFinalTImeSeconds FinalTimeSeconds)
  (Utilities|FlowControl|Delay 5.0)
  (bind _returnvalue_2 (UserInterface|CreateWidget "/Game/UI/Widgets/WBP_MissionEndTransition.WBP_MissionEndTransition_C" _returnvalue))
  (bind _output_get (Variables|Default|SetMissionEndTransitionRef _returnvalue_2))
  (UserInterface|Viewport|AddtoViewport _output_get 40)
  (UserInterface|Animation|PlayAnimation (Variables|Default|GetMissionEndTransitionRef) (Variables|/Game/UI/Widgets/WBP_MissionEndTransition.WBP_MissionEndTransition_C|GetAnim_FadeToResult (Variables|Default|GetMissionEndTransitionRef)) 0.0 1 "Forward" 1.0 false)
  (Utilities|FlowControl|Delay 1.0)
  (bind _returnvalue_3 (UserInterface|CreateWidget "/Game/UI/Widgets/WBP_MissionResult.WBP_MissionResult_C" _returnvalue self (Variables|Default|GetCachedMissionSuccess) (Variables|Default|GetCachedFinalScore) (Variables|Default|GetCachedFinalUsedDrones) (Variables|Default|GetCachedFinalTImeSeconds) "/Game/UI/Widgets/WBP_MissionObjective.WBP_MissionObjective_C"))
  (UserInterface|Viewport|AddtoViewport _returnvalue_3 50)
  (Widget|RemovefromParent (Variables|Default|GetMissionEndTransitionRef))
  (Game|SetGamePaused true)
  (Variables|/Script/Engine.PlayerController|SetbShowMouseCursor _returnvalue true)
  (Input|SetInputModeUIOnly _returnvalue _returnvalue_3 "DoNotLock"))

(fn ConstructionScript)