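; Player controller for the FPV game that handles the mission briefing screen and the pause menu.
; Shortly after BeginPlay it finds the mission scenario controller, shows WBP_LoadingScreen with it, pauses the game and sets BriefingOpen.
; Outside briefings, PauseMenu input closes any active submenu first, otherwise toggles the pause widget, which also receives the mission controller.
; Opening and closing the menu switches pause state, input mode and cursor visibility.
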(event Custom|ClosePauseMenu
  (Utilities|IsValid (Variables|Default|GetPauseMenuWidget)
    (:Is%20Valid
      (Widget|RemovefromParent (Variables|Default|GetPauseMenuWidget))
      (Variables|Default|SetPauseMenuWidget 0)
      (Game|SetGamePaused false)
      (Input|SetInputModeGameOnly self)
      (Variables|Default|SetbShowMouseCursor false))))

(event EventBeginPlay
  (Development|PrintString "Hello")
  (Utilities|FlowControl|Delay 0.1)
  (bind _outactors (Actor|GetAllActorsOfClass "/Script/Diploma.MissionScenarioController"))
  (if (> (Utilities|Array|Length _outactors) 0)
    (bind _asbp_mission_scenario_controller (Utilities|Casting|CastToBP_MissionScenarioController (Utilities|Array|Get(acopy) _outactors)))
    (bind _returnvalue (UserInterface|CreateWidget "/Game/UI/Widgets/WBP_LoadingScreen.WBP_LoadingScreen_C" self _asbp_mission_scenario_controller))
    (UserInterface|Viewport|AddtoViewport _returnvalue 100)
    (Variables|Default|SetbBriefingOpen true)
    (Variables|Default|SetbShowMouseCursor true)
    (Input|SetInputModeUIOnly self _returnvalue "DoNotLock")
    (Game|SetGamePaused true)))

(event EventTick
  (params (DeltaSeconds :type Float%20%28single-precision%29)))

(event Input|ActionEvents|InputActionPauseMenu
  (params (Key :type Key%20Structure :default "None"))
  (:Pressed
    (if (not (Variables|Default|GetbBriefingOpen))
      (bind _returnvalue (Actor|GetActorOfClass "/Game/Maps/BP_MissionScenarioController.BP_MissionScenarioController_C"))
      (Utilities|IsValid _returnvalue
        (:Is%20Valid
          (Utilities|IsValid (Variables|Default|GetActivePauseSubmenu)
            (:Is%20Valid
              (Widget|RemovefromParent (Variables|Default|GetActivePauseSubmenu))
              (Variables|Default|SetActivePauseSubmenu 0)
              (Utilities|IsValid (Variables|Default|GetPauseMenuWidget)
                (:Is%20Valid
                  (Widget|SetIsEnabled (Variables|Default|GetPauseMenuWidget) true)
                  (Input|SetInputModeGameandUI self (Variables|Default|GetPauseMenuWidget) "DoNotLock" false)
                  (Variables|Default|SetbShowMouseCursor true))))
            (:Is%20Not%20Valid
              (Development|PrintString "Paused")
              (Utilities|IsValid (Variables|Default|GetPauseMenuWidget)
                (:Is%20Valid
                  (CallFunction|ClosePauseMenu))
                (:Is%20Not%20Valid
                  (bind _returnvalue_2 (Actor|GetActorOfClass "/Game/Maps/BP_MissionScenarioController.BP_MissionScenarioController_C"))
                  (bind _returnvalue_3 (UserInterface|CreateWidget (Variables|Default|GetPauseMenuClass) self _returnvalue_2))
                  (bind _output_get (Variables|Default|SetPauseMenuWidget _returnvalue_3))
                  (UserInterface|Viewport|AddtoViewport _output_get 50)
                  (Game|SetGamePaused true)
                  (Input|SetInputModeGameandUI self (Variables|Default|GetPauseMenuWidget) "DoNotLock" false)
                  (Variables|Default|SetbShowMouseCursor true))))))))))

(fn ConstructionScript)